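; Player state for a multiplayer card game that pushes player name, room name, dealt cards and tags to the local HUD's main card widget.
; RepNotifies on name, room name and IsFirst trigger the UI updates, which use short delays before reaching the HUD.
; In the Prepare turn it shows the next player's cards, found by wrapping through PlayerArray, then asks the game state to switch to Drawing Cards, which only prints.
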(event `self.ReceiveBeginPlay`)

(event `UpdateName_Mitli`
  (params (BP_CardPlayerState :type "/Game/CWB2/Player/BP_CardPlayerState Object Reference"))
  (bind _returnvalue (`GameplayStatics.GetPlayerController` 0))
  ;[1 1 1] 显示本地的名称
  (`KismetSystemLibrary.Delay` 0.05)
  (if (== (`Controller.PlayerState` _returnvalue) BP_CardPlayerState)
    (bind _asbp_card_hud (cast `/Game/CWB2/UI/BP_CardHUD` (`PlayerController.GetHUD` _returnvalue)))
    (bind _w_cardmain (`/Game/CWB2/UI/BP_CardHUD.W_CardMain` _asbp_card_hud))
    (`/Engine/EditorBlueprintResources/StandardMacros.IsValid` _w_cardmain
      (:`Is Valid`
        (`/Game/CWB2/UI/Card/W_CardMain.SetPlayerNameText` _w_cardmain (`|FormatText` "我是：{0} " (`self.Name`)))))))

(event `UpdateRoomName_Mitli`
  (params (BP_CardPlayerState :type "/Game/CWB2/Player/BP_CardPlayerState Object Reference"))
  ;[1 1 1] 显示房间名字
  (`KismetSystemLibrary.Delay` 0.05)
  (bind _asbp_card_hud (cast `/Game/CWB2/UI/BP_CardHUD` (`PlayerController.GetHUD` (`GameplayStatics.GetPlayerController` 0))))
  (bind _w_cardmain (`/Game/CWB2/UI/BP_CardHUD.W_CardMain` _asbp_card_hud))
  (`/Engine/EditorBlueprintResources/StandardMacros.IsValid` _w_cardmain
    (:`Is Valid`
      (`/Game/CWB2/UI/Card/W_CardMain.SetRoomNameText` _w_cardmain (`|FormatText` "{0} 的房间" (`self.RoomName`))))))

(event `UpdateCards_Mutli`
  ;[1 1 1] 首次发拍到卡组
  (`|ExecutionSequence`
    (:`then_0`
      (`KismetSystemLibrary.Delay` 0.02)
      (bind _bp_card_hud (`self.GetBPHUD`))
      (bind _asbp_card_player_state (cast `/Game/CWB2/Player/BP_CardPlayerState` (`Controller.PlayerState` (`GameplayStatics.GetPlayerController` 0))))
      (for _array_element (`/Game/CWB2/Player/BP_CardPlayerState.Cards` _asbp_card_player_state)
        (bind _w_cardmain (`/Game/CWB2/UI/BP_CardHUD.W_CardMain` _bp_card_hud))
        (`/Game/CWB2/UI/Card/W_CardMain.AddChildtoPlayerCardsScrollBox` _w_cardmain _array_element true 0 null))
      (`/Game/CWB2/UI/Card/W_CardMain.All Person Is Ready` _w_cardmain))
    (:`then_1`
      (`KismetSystemLibrary.PrintString` (`KismetStringLibrary.Concat_StrStr` "这里走")))))

(event `UpdateTurnType_Client`
  (params (TurnType :type "/Game/CWB2/Data/E_TurnType Enum" :default "NewEnumerator0"))
  (switch `/Game/CWB2/Data/E_TurnType` TurnType
    (:`NewEnumerator1`
      (set `self.NextPlayer_PS` null)
      (bind _next (`self.GetNextPlayer`))
      (set `self.NextPlayer_PS` _next)
      (`KismetSystemLibrary.Delay` 0.02)
      (bind _bp_card_hud (`self.GetBPHUD`))
      (bind _w_cardmain (`/Game/CWB2/UI/BP_CardHUD.W_CardMain` _bp_card_hud))
      (`/Engine/EditorBlueprintResources/StandardMacros.IsValid` _w_cardmain
        (:`Is Valid`
          (`/Game/CWB2/UI/Card/W_CardMain.PlayShowOtherCardsAnimation` _w_cardmain)
          (`/Game/CWB2/UI/Card/W_CardMain.UpdateOtherCardsScrollBox` _w_cardmain (`self.NextPlayer_PS`))
          (`self.ChangeTurn` "NewEnumerator2"))))
    (:`NewEnumerator2`
      (`KismetSystemLibrary.PrintString` "抽牌阶段"))))

(event `AddNewTag_Mutli`
  (params (Text :type Text))
  (bind _bp_card_hud (`self.GetBPHUD`))
  (bind _w_cardmain (`/Game/CWB2/UI/BP_CardHUD.W_CardMain` _bp_card_hud))
  (`/Engine/EditorBlueprintResources/StandardMacros.IsValid` _w_cardmain
    (:`Is Valid`
      (`/Game/CWB2/UI/Card/W_CardMain.AddNewTag` _w_cardmain Text))))

(fn `ChangeTurn`
  (params (`New Turn` :type "/Game/CWB2/Data/E_TurnType Enum" :default "NewEnumerator0"))
  (bind _asbp_card_gs (cast `/Game/CWB2/GameMode/BP_CardGS` (`GameplayStatics.GetGameState`)))
  (cast `/Game/CWB2/Player/BP_CardPlayerState` (`Controller.PlayerState` (`GameplayStatics.GetPlayerController` 0)))
  (`/Game/CWB2/GameMode/BP_CardGS.FinishAndChangeTurn` _asbp_card_gs `New Turn` self))

(fn `GetBPHUD`
  (returns (`BP Card HUD` :type "/Game/CWB2/UI/BP_CardHUD Object Reference"))
  (bind _asbp_card_hud (cast `/Game/CWB2/UI/BP_CardHUD` (`PlayerController.GetHUD` (`GameplayStatics.GetPlayerController` 0))))
  (return _asbp_card_hud))

(fn `GetNextPlayer`
  (returns (Next :type "/Game/CWB2/Player/BP_CardPlayerState Object Reference"))
  (locals (TempPS :type "/Game/CWB2/Player/BP_CardPlayerState Object Reference"))
  (bind _playerarray (`GameStateBase.PlayerArray` (`GameplayStatics.GetGameState`)))
  (bind _output (`|GetArrayItem` (`GameStateBase.PlayerArray` (`GameplayStatics.GetGameState`))))
  (set `local.TempPS` null)
  (for (_array_element _array_index) _playerarray
    (if (== _array_element (`Controller.PlayerState` (`GameplayStatics.GetPlayerController` 0)))
      (bind _output_2 (`|GetArrayItem` _playerarray (+ _array_index 1)))
      (`/Engine/EditorBlueprintResources/StandardMacros.IsValid` _output_2
        (:`Is Valid`
          (bind _asbp_card_player_state (cast `/Game/CWB2/Player/BP_CardPlayerState` _output_2))
          (set `local.TempPS` _asbp_card_player_state)
          (break))
        (:`Is Not Valid`
          (`/Engine/EditorBlueprintResources/StandardMacros.IsValid` _output
            (:`Is Valid`
              (bind _asbp_card_player_state_2 (cast `/Game/CWB2/Player/BP_CardPlayerState` _output))
              (set `local.TempPS` _asbp_card_player_state_2)
              (break)))))))
  (return (`local.TempPS`)))

(fn `OnRep_IsFirst`
  (`self.UpdateCards_Mutli`))

(fn `OnRep_Name`
  (`self.UpdateName_Mitli` self))

(fn `OnRep_RoomName`
  (`self.UpdateRoomName_Mitli` self))

(fn `UserConstructionScript`)