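; Player state for the multiplayer room lobby, holding each player's name, room name and ready state.
; Name and ready edits route through server events to BP_RoomGM; OnRep functions refresh BP_RoomHUD widgets, backed by a timer that rebuilds mismatched player lists.
; CopyProperties passes names to BP_CardPlayerState and records players and their count in the game instance.
; OpenNewLevel server-travels to the card map on authority.
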(event `self.ReceiveBeginPlay`
  (`KismetSystemLibrary.K2_SetTimerDelegate` (delegate `CheckPlayerNumber`) 1.0 true))

(event `self.ReceiveTick`
  (params (DeltaSeconds :type "Float (single-precision)")))

(event `CheckPlayerNumber`
  (bind _asbp_room_hud (cast `/Game/CWB2/UI/BP_RoomHUD` (`PlayerController.GetHUD` (`GameplayStatics.GetPlayerController` 0))))
  (bind _w_inroom (`/Game/CWB2/UI/BP_RoomHUD.W_InRoom` _asbp_room_hud))
  (`/Engine/EditorBlueprintResources/StandardMacros.IsValid` _w_inroom
    (:`Is Valid`
      (if (not (== (`KismetArrayLibrary.Array_Length` (`PanelWidget.GetAllChildren` (`/Game/CWB2/UI/InRoom/W_InRoom.PlayerItem_ScrollBox` _w_inroom))) (`KismetArrayLibrary.Array_Length` (`GameStateBase.PlayerArray` (`GameplayStatics.GetGameState`)))))
        (`/Game/CWB2/UI/BP_RoomHUD.Update Player List` _asbp_room_hud null)))))

(event `UpdateRoomName_Mitli`
  (`KismetSystemLibrary.Delay` 0.02)
  (bind _asbp_room_hud (cast `/Game/CWB2/UI/BP_RoomHUD` (`PlayerController.GetHUD` (`GameplayStatics.GetPlayerController` 0))))
  (bind _w_inroom (`/Game/CWB2/UI/BP_RoomHUD.W_InRoom` _asbp_room_hud))
  (`/Engine/EditorBlueprintResources/StandardMacros.IsValid` _w_inroom
    (:`Is Valid`
      (`TextBlock.SetText` (`/Game/CWB2/UI/InRoom/W_InRoom.RoomNameText` _w_inroom) (`|FormatText` "{0} 的房间" (`self.RoomName`))))))

(event `UpdateName_Mitli`
  (params (BP_RoomPlayerState :type "/Game/CWB2/Player/BP_RoomPlayerState Object Reference"))
  (bind _name (`/Game/CWB2/Player/BP_RoomPlayerState.Name` BP_RoomPlayerState))
  (`KismetSystemLibrary.Delay` 0.02)
  (bind _asbp_room_hud (cast `/Game/CWB2/UI/BP_RoomHUD` (`PlayerController.GetHUD` (`GameplayStatics.GetPlayerController` 0))))
  (bind _w_inroom (`/Game/CWB2/UI/BP_RoomHUD.W_InRoom` _asbp_room_hud))
  (`/Engine/EditorBlueprintResources/StandardMacros.IsValid` _w_inroom
    (:`Is Valid`
      (bind (_finded1 _tempplayeritem1) (`/Game/CWB2/UI/BP_RoomHUD.Find Player Item` _asbp_room_hud BP_RoomPlayerState))
      (if _finded1
        (`/Game/CWB2/UI/InRoom/W_PlayerItem.SetPlayerName` _tempplayeritem1 _name))
      (if (== (`Controller.PlayerState` (`GameplayStatics.GetPlayerController` 0)) BP_RoomPlayerState)
        (`TextBlock.SetText` (`/Game/CWB2/UI/InRoom/W_InRoom.LocalPlayerNameTextBlock` _w_inroom) _name)))))

(event `self.ReceiveCopyProperties`
  (params (NewPlayerState :type "PlayerState Object Reference"))
  (bind _asbp_card_player_state (cast `/Game/CWB2/Player/BP_CardPlayerState` NewPlayerState))
  (set `/Game/CWB2/Player/BP_CardPlayerState.Name` (`self.Name`) _asbp_card_player_state)
  (set `/Game/CWB2/Player/BP_CardPlayerState.RoomName` (`self.RoomName`) _asbp_card_player_state)
  (bind _asbp_create_room_gi (cast `/Game/CWB2/GameMode/BP_CreateRoomGI` (`GameplayStatics.GetGameInstance`)))
  (`/Game/CWB2/GameMode/BP_CreateRoomGI.AddNewPlayer` _asbp_create_room_gi (make `/Game/CWB2/Data/BPS_PlayerInfo` _asbp_card_player_state (`self.Name`) (`self.RoomName`)))
  (`self.RecordTheNumberOfPlayers` _asbp_create_room_gi)
  (`parent.ReceiveCopyProperties` NewPlayerState))

(event `UpdatePlayerItem_Mutli`
  (`KismetSystemLibrary.Delay` 0.02)
  (bind _asbp_room_hud (cast `/Game/CWB2/UI/BP_RoomHUD` (`PlayerController.GetHUD` (`GameplayStatics.GetPlayerController` 0))))
  (`/Game/CWB2/UI/BP_RoomHUD.Update Player List` _asbp_room_hud null))

(event `UpdateName`
  (params (BP_RoomPlayerState :type "/Game/CWB2/Player/BP_RoomPlayerState Object Reference") (Text :type Text))
  (`/Engine/EditorBlueprintResources/ActorMacros.Switch Has Authority`
    (:`Authority`
      (bind _asbp_room_gm (cast `/Game/CWB2/GameMode/BP_RoomGM` (`GameplayStatics.GetGameMode`)))
      (`/Game/CWB2/GameMode/BP_RoomGM.UpdateName` _asbp_room_gm BP_RoomPlayerState Text)
      (`/Game/CWB2/GameMode/BP_RoomGM.UpdateRoomName` _asbp_room_gm BP_RoomPlayerState Text))
    (:`Remote`
      (`self.UpdateName_Server` BP_RoomPlayerState Text))))

(event `UpdateName_Server`
  (params (BP_RoomPlayerState :type "/Game/CWB2/Player/BP_RoomPlayerState Object Reference") (Text :type Text))
  (bind _asbp_room_gm (cast `/Game/CWB2/GameMode/BP_RoomGM` (`GameplayStatics.GetGameMode`)))
  (`/Game/CWB2/GameMode/BP_RoomGM.UpdateName` _asbp_room_gm BP_RoomPlayerState Text))

(event `UpdateIsReady`
  (params (BP_RoomPlayerState :type "/Game/CWB2/Player/BP_RoomPlayerState Object Reference") (IsReady :type Boolean))
  (`/Engine/EditorBlueprintResources/ActorMacros.Switch Has Authority`
    (:`Authority`
      (bind _asbp_room_gm (cast `/Game/CWB2/GameMode/BP_RoomGM` (`GameplayStatics.GetGameMode`)))
      (`/Game/CWB2/GameMode/BP_RoomGM.UpdateIsReady` _asbp_room_gm BP_RoomPlayerState IsReady))
    (:`Remote`
      (`self.UpdateIsReady_Server` BP_RoomPlayerState IsReady))))

(event `UpdateIsReady_Server`
  (params (BP_RoomPlayerState :type "/Game/CWB2/Player/BP_RoomPlayerState Object Reference") (IsReady :type Boolean))
  (bind _asbp_room_gm (cast `/Game/CWB2/GameMode/BP_RoomGM` (`GameplayStatics.GetGameMode`)))
  (`/Game/CWB2/GameMode/BP_RoomGM.UpdateIsReady` _asbp_room_gm BP_RoomPlayerState IsReady))

(event `UpdateIsReady_Mutli`
  (params (BP_RoomPlayerState :type "/Game/CWB2/Player/BP_RoomPlayerState Object Reference"))
  (bind _asbp_room_hud (cast `/Game/CWB2/UI/BP_RoomHUD` (`PlayerController.GetHUD` (`GameplayStatics.GetPlayerController` 0))))
  (bind (_finded1 _tempplayeritem1) (`/Game/CWB2/UI/BP_RoomHUD.Find Player Item` _asbp_room_hud BP_RoomPlayerState))
  (if _finded1
    (`/Game/CWB2/UI/InRoom/W_PlayerItem.SetIsReady` _tempplayeritem1 (`self.IsReady`))))

(event `OpenNewLevel`
  (`/Engine/EditorBlueprintResources/ActorMacros.Switch Has Authority`
    (:`Authority`
      (`KismetSystemLibrary.ExecuteConsoleCommand` "ServerTravel /Game/CWB2/Maps/L_CardMap?listen" (`GameplayStatics.GetPlayerController` 0)))))

(fn `OnRep_IsReady`
  (`self.UpdateIsReady_Mutli` self))

(fn `OnRep_Name`
  (`self.UpdateName_Mitli` self))

(fn `OnRep_NeedUpdate`
  (`self.UpdatePlayerItem_Mutli`))

(fn `OnRep_RoomName`
  (`self.UpdateRoomName_Mitli`))

(fn `RecordTheNumberOfPlayers`
  (params (GI :type "/Game/CWB2/GameMode/BP_CreateRoomGI Object Reference"))
  (locals (Num :type Integer))
  (set `local.Num` 0)
  (for _array_element (`GameStateBase.PlayerArray` (`GameplayStatics.GetGameState`))
    (cast `/Game/CWB2/Player/BP_RoomPlayerState` _array_element)
    (`/Engine/EditorBlueprintResources/StandardMacros.IncrementInt` (`local.Num`)))
  (`KismetSystemLibrary.PrintString` (`KismetStringLibrary.Conv_IntToString` (`local.Num`)))
  (`/Game/CWB2/GameMode/BP_CreateRoomGI.SetPlayerNumbers` GI (`local.Num`))
  (return))

(fn `UserConstructionScript`)