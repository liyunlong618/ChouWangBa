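; Game mode for a multiplayer card game, handling match start, dealing and turn changes.
; A looping timer copies names and room names from the game instance into player states until all expected players load.
; It then deals equal random-sized hands, gives one random player an extra card and a marked card, and has GameState show a countdown.
; After the countdown that player enters the prepare turn; turn changes are broadcast through dispatchers.
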(event `self.ReceiveBeginPlay`
  (bind _returnvalue (`KismetSystemLibrary.K2_SetTimerDelegate` (delegate `SetName`) 0.1 true))
  (set `self.SetNameTimerHandle` _returnvalue))

(event `SetName`
  (bind _returnvalue (`KismetArrayLibrary.Array_Length` (`GameStateBase.PlayerArray` (`GameplayStatics.GetGameState`))))
  (for _array_element (`GameStateBase.PlayerArray` (`GameplayStatics.GetGameState`))
    (bind _asbp_card_player_state (cast `/Game/CWB2/Player/BP_CardPlayerState` _array_element))
    (bind _asbp_create_room_gi (cast `/Game/CWB2/GameMode/BP_CreateRoomGI` (`GameplayStatics.GetGameInstance`)))
    (bind (_find1 _finditem1) (`/Game/CWB2/GameMode/BP_CreateRoomGI.GetInfoByPS` _asbp_create_room_gi _asbp_card_player_state))
    (if _find1
      (set `/Game/CWB2/Player/BP_CardPlayerState.Name` (`.Name_5_BCAAC94F4A09C99DDA45A4A86F763C20` (break `/Game/CWB2/Data/BPS_PlayerInfo` _finditem1)) (break `/Game/CWB2/Data/BPS_PlayerInfo` _finditem1))
      (set `/Game/CWB2/Player/BP_CardPlayerState.RoomName` (`.RoomName_12_407143CD4DA9ABD93E5E67AE55E38D29` (break `/Game/CWB2/Data/BPS_PlayerInfo` _finditem1)) (break `/Game/CWB2/Data/BPS_PlayerInfo` _finditem1))))
  (bind _asbp_create_room_gi_2 (cast `/Game/CWB2/GameMode/BP_CreateRoomGI` (`GameplayStatics.GetGameInstance`)))
  (bind _playernumbers (`/Game/CWB2/GameMode/BP_CreateRoomGI.GetPlayerNumbers` _asbp_create_room_gi_2))
  (if (>= _returnvalue _playernumbers)
    (`|ExecutionSequence`
      (:`then_0`
        (`KismetSystemLibrary.Delay` 2.0)
        (`|ExecutionSequence`
          (:`then_0`
            (`self.Dealing Cards`)
            (`KismetSystemLibrary.K2_ClearAndInvalidateTimerHandle` (`self.SetNameTimerHandle`)))
          (:`then_1`
            ;[1 1 1] 倒计时UI
            (bind _asbp_card_gs (cast `/Game/CWB2/GameMode/BP_CardGS` (`GameplayStatics.GetGameState`)))
            (`/Game/CWB2/GameMode/BP_CardGS.CreateReadyToStartUI` _asbp_card_gs))))
      (:`then_1`
        (`KismetSystemLibrary.PrintString` "加载测试：全都加载完了")))
    (else
      (`KismetSystemLibrary.PrintString` (`KismetStringLibrary.Concat_StrStr` "加载测试：有人没加载完" (`KismetStringLibrary.Conv_IntToString` _playernumbers) "/" (`KismetStringLibrary.Conv_IntToString` _returnvalue))))))

(event `self.ReceiveTick`
  (params (DeltaSeconds :type "Float (single-precision)")))

(event `FinishPlayNumberAnimation`
  ;[1 1 1] 完成了播放倒计时动画，切换第一个玩家为 开始回合
  (bind _findps (`self.FindFirstPlayer`))
  (`self.UpdatePlayerTurnType` _findps "NewEnumerator1"))

(event `ChangeTurn`
  (params (TurnType :type "/Game/CWB2/Data/E_TurnType Enum" :default "NewEnumerator0") (BP_CardPlayerState :type "/Game/CWB2/Player/BP_CardPlayerState Object Reference"))
  (`self.UpdatePlayerTurnType` BP_CardPlayerState TurnType))

(event `AddNewTag`
  (params (TurnType :type "/Game/CWB2/Data/E_TurnType Enum" :default "NewEnumerator0") (BP_CardPlayerState :type "/Game/CWB2/Player/BP_CardPlayerState Object Reference"))
  (`KismetSystemLibrary.Delay` 0.2)
  (bind _asbp_card_gs (cast `/Game/CWB2/GameMode/BP_CardGS` (`GameplayStatics.GetGameState`))
    (:`then`
      (`KismetSystemLibrary.PrintString` "拿到GS")
      (`/Game/CWB2/GameMode/BP_CardGS.AddNewTag` _asbp_card_gs TurnType BP_CardPlayerState))
    (:`CastFailed`
      (`KismetSystemLibrary.PrintString` "没拿到GS"))))

(fn `Dealing Cards`
  (locals (TempCards :type "Array of Integer") (TempNum :type Integer :default 0))
  (bind _playerarray (`GameStateBase.PlayerArray` (`GameplayStatics.GetGameState`)))
  (set `local.TempNum` (`KismetMathLibrary.RandomIntegerInRange` 3 8))
  (for _index (range (+ (`KismetArrayLibrary.Array_LastIndex` _playerarray) 1))
    (bind _asbp_card_player_state (cast `/Game/CWB2/Player/BP_CardPlayerState` (`|GetArrayItem` _playerarray _index)))
    (for _ (range (+ (`local.TempNum`) 1))
      (`KismetArrayLibrary.Array_Add` (`/Game/CWB2/Player/BP_CardPlayerState.Cards` _asbp_card_player_state))))
  (bind _asbp_card_player_state_2 (cast `/Game/CWB2/Player/BP_CardPlayerState` (`KismetArrayLibrary.Array_Random` _playerarray)))
  (bind _cards (`/Game/CWB2/Player/BP_CardPlayerState.Cards` _asbp_card_player_state_2))
  (`KismetArrayLibrary.Array_Add` _cards)
  (`KismetArrayLibrary.Array_Set` _cards (`.OutIndex` (`KismetArrayLibrary.Array_Random` _cards)) 1 true)
  (set `/Game/CWB2/Player/BP_CardPlayerState.IsFirst` true _asbp_card_player_state_2)
  (`|ExecutionSequence`
    (:`then_0`
      (return))
    (:`then_1`
      (`KismetSystemLibrary.PrintString` "执行完发牌"))))

(fn `FindFirstPlayer`
  (returns (FindPS :type "/Game/CWB2/Player/BP_CardPlayerState Object Reference"))
  (locals (TempFindPS :type "/Game/CWB2/Player/BP_CardPlayerState Object Reference"))
  (set `local.TempFindPS` null)
  (for _array_element (`GameStateBase.PlayerArray` (`GameplayStatics.GetGameState`))
    (bind _asbp_card_player_state (cast `/Game/CWB2/Player/BP_CardPlayerState` _array_element))
    (if (`/Game/CWB2/Player/BP_CardPlayerState.IsFirst` _asbp_card_player_state)
      (set `local.TempFindPS` _asbp_card_player_state)
      (break)))
  (return (`local.TempFindPS`)))

(fn `UpdatePlayerTurnType`
  (params (PS :type "/Game/CWB2/Player/BP_CardPlayerState Object Reference") (TurnType :type "/Game/CWB2/Data/E_TurnType Enum" :default "NewEnumerator0"))
  (locals (TempFindPS :type "Object Object Reference"))
  (bind _output_get (set `/Game/CWB2/Player/BP_CardPlayerState.TurnType` TurnType PS))
  (`self.ChangeTurn_EventDispatcher` PS _output_get)
  (`self.AddNewTag_EventDispatcher` (`|FormatText` "玩家{0}进入{1}" (`/Game/CWB2/Player/BP_CardPlayerState.Name` PS) (select `/Game/CWB2/Data/E_TurnType` _output_get :`NewEnumerator0` "回合开始" :`NewEnumerator1` "准备阶段" :`NewEnumerator2` "抽牌回合" :`NewEnumerator3` "结束抽牌" :`NewEnumerator4` "回合结束" :!type "Text")))
  (return))

(fn `UserConstructionScript`)