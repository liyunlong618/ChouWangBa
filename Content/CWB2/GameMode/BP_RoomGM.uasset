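; Game mode for a multiplayer room lobby that sets up player and room names as players join.
; BeginPlay applies the name saved in the game instance to the first player's state, treated as the host.
; PostLogin names other players by ID, copies the host's name as RoomName, refreshes player items through BP_RoomGS and increments the host's NeedUpdate counter.
; Custom events write name, room name and ready changes into a given BP_RoomPlayerState.
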(event `self.ReceiveBeginPlay`
  (bind _asbp_create_room_gi (cast `/Game/CWB2/GameMode/BP_CreateRoomGI` (`GameplayStatics.GetGameInstance`)))
  (bind _asbp_room_player_state (cast `/Game/CWB2/Player/BP_RoomPlayerState` (`Controller.PlayerState` (`GameplayStatics.GetPlayerController` 0))))
  (set `/Game/CWB2/Player/BP_RoomPlayerState.Name` (`/Game/CWB2/GameMode/BP_CreateRoomGI.Name` _asbp_create_room_gi) _asbp_room_player_state)
  (bind _asbp_room_player_state_2 (cast `/Game/CWB2/Player/BP_RoomPlayerState` (`GameplayStatics.GetPlayerState` 0)))
  (set `/Game/CWB2/Player/BP_RoomPlayerState.RoomName` (`/Game/CWB2/Player/BP_RoomPlayerState.Name` _asbp_room_player_state_2) _asbp_room_player_state))

(event `self.K2_PostLogin`
  (params (NewPlayer :type "PlayerController Object Reference"))
  (bind _playerstate (`Controller.PlayerState` NewPlayer))
  (if (== _playerstate (`GameplayStatics.GetPlayerState` 0))
    (`KismetSystemLibrary.PrintString` "服务器进来了")
    (bind _asbp_room_gs (cast `/Game/CWB2/GameMode/BP_RoomGS` (`GameplayStatics.GetGameState`)))
    (`/Game/CWB2/GameMode/BP_RoomGS.UpdatePlayerItem` _asbp_room_gs)
    (bind _asbp_room_player_state (cast `/Game/CWB2/Player/BP_RoomPlayerState` (`GameplayStatics.GetPlayerState` 0)))
    (set `/Game/CWB2/Player/BP_RoomPlayerState.RoomName` (`/Game/CWB2/Player/BP_RoomPlayerState.Name` _asbp_room_player_state) _asbp_room_player_state)
    (`/Engine/EditorBlueprintResources/StandardMacros.IncrementInt` (`/Game/CWB2/Player/BP_RoomPlayerState.NeedUpdate` _asbp_room_player_state))
    (else
      (`KismetSystemLibrary.PrintString` "玩家进来了")
      (bind _asbp_room_player_state_2 (cast `/Game/CWB2/Player/BP_RoomPlayerState` _playerstate))
      (set `/Game/CWB2/Player/BP_RoomPlayerState.Name` (`|FormatText` "玩家{0}" (`KismetTextLibrary.Conv_IntToText` (`PlayerState.PlayerId` _playerstate))) _asbp_room_player_state_2)
      (bind _asbp_room_player_state_3 (cast `/Game/CWB2/Player/BP_RoomPlayerState` (`GameplayStatics.GetPlayerState` 0)))
      (set `/Game/CWB2/Player/BP_RoomPlayerState.RoomName` (`/Game/CWB2/Player/BP_RoomPlayerState.Name` _asbp_room_player_state_3) _asbp_room_player_state_2)
      (bind _asbp_room_gs_2 (cast `/Game/CWB2/GameMode/BP_RoomGS` (`GameplayStatics.GetGameState`)))
      (`/Game/CWB2/GameMode/BP_RoomGS.UpdatePlayerItem` _asbp_room_gs_2)
      (`/Engine/EditorBlueprintResources/StandardMacros.IncrementInt` (`/Game/CWB2/Player/BP_RoomPlayerState.NeedUpdate` _asbp_room_player_state_3)))))

(event `UpdateName`
  (params (BP_RoomPlayerState :type "/Game/CWB2/Player/BP_RoomPlayerState Object Reference") (Text :type Text))
  (set `/Game/CWB2/Player/BP_RoomPlayerState.Name` Text BP_RoomPlayerState)
  (`KismetSystemLibrary.PrintString` "GM"))

(event `UpdateRoomName`
  (params (BP_RoomPlayerState :type "/Game/CWB2/Player/BP_RoomPlayerState Object Reference") (Text :type Text))
  (set `/Game/CWB2/Player/BP_RoomPlayerState.RoomName` Text BP_RoomPlayerState))

(event `UpdateIsReady`
  (params (BP_RoomPlayerState :type "/Game/CWB2/Player/BP_RoomPlayerState Object Reference") (IsReady :type Boolean))
  (set `/Game/CWB2/Player/BP_RoomPlayerState.IsReady` IsReady BP_RoomPlayerState))

(fn `UserConstructionScript`)