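; Room-creation game instance, going by its name, that holds a PlayerInfos list of per-player records.
; AddNewPlayer appends a record to the list.
; GetInfoByPS searches the list linearly for the first record whose player state has the same PlayerId as the given one, returning a found flag and that record.
; Matching uses the ID rather than the player state reference.
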(fn `AddNewPlayer`
  (params (NewItem :type "/Game/CWB2/Data/BPS_PlayerInfo Structure (by ref)"))
  (`KismetArrayLibrary.Array_Add` (`self.PlayerInfos`) NewItem))

(fn `GetInfoByPS`
  (params (PS :type "/Game/CWB2/Player/BP_CardPlayerState Object Reference"))
  (returns (Find1 :type Boolean) (FindItem1 :type "/Game/CWB2/Data/BPS_PlayerInfo Structure"))
  (locals (FindItem :type "/Game/CWB2/Data/BPS_PlayerInfo Structure") (Find :type Boolean))
  (set `local.Find` false)
  (for _array_element (`self.PlayerInfos`)
    (if (== (`PlayerState.PlayerId` (`.PS_9_C276AD9342F100210C7BC4986E20827B` (break `/Game/CWB2/Data/BPS_PlayerInfo` _array_element))) (`PlayerState.PlayerId` PS))
      (set `local.FindItem` _array_element)
      (set `local.Find` true)
      (break)))
  (return (`local.Find`) (`local.FindItem`)))